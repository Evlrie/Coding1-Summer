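; BP_CanofBeans is a holdable can of beans pickup for the custom third-person character.
; Overlapping its trigger asks the character to pick it up, and Pickup attaches its root to the hand_r socket of the supplied mesh.
; Drop detaches it and enables physics and collision on the can.
; PrimaryAction consumes it, only printing a health message, clearing the character's HeldItem and destroying the actor.
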(event OnComponentBeginOverlap(PickupTrigger)
  (params (OverlappedComponent :type Primitive%20Component%20Object%20Reference) (OtherActor :type Actor%20Object%20Reference) (OtherComp :type Primitive%20Component%20Object%20Reference) (OtherBodyIndex :type Integer) (bFromSweep :type Boolean) (SweepResult :type Hit%20Result%20Structure%20%28by%20ref%29))
  (bind _ascoding_1third_person_custom (Utilities|Casting|CastToCoding1ThirdPersonCustom OtherActor))
  (Default|TrytoPickUP _ascoding_1third_person_custom self))

(event EventBeginPlay)

(event Collision|EventActorBeginOverlap
  (params (OtherActor :type Actor%20Object%20Reference)))

(event EventTick
  (params (DeltaSeconds :type Float%20%28single-precision%29)))

(event EventPickup
  (params (ParentMesh :type Skeletal%20Mesh%20Component%20Object%20Reference))
  (Transformation|AttachComponentToComponent (Variables|Default|GetDefaultSceneRoot) ParentMesh "hand_r" "SnapToTarget" "KeepRelative" "KeepRelative" true))

(event EventDrop
  (Transformation|DetachFromComponent (Variables|Default|GetDefaultSceneRoot) "KeepRelative" "KeepRelative" "KeepRelative" true)
  (Physics|SetSimulatePhysics (Variables|Default|Getcan) true)
  (Collision|SetCollisionEnabled (Variables|Default|Getcan) "QueryAndPhysics"))

(event EventPrimaryAction
  (params (Ref_ThirdPersonCharCustom :type Coding%201%20Third%20Person%20Custom%20Object%20Reference))
  (Development|PrintString "+10 health" true true "(R=0.292796,G=1.000000,B=0.161611,A=1.000000)")
  (Variables|/Game/Blueprints/Coding1ThirdPersonCustom.Coding1ThirdPersonCustom_C|SetHeldItem Ref_ThirdPersonCharCustom 0)
  (Actor|DestroyActor))

(fn ConstructionScript)