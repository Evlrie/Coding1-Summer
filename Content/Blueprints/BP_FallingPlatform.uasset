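; Falling platform that drops when the player character steps into its box trigger, then returns to where it started.
; After a one-second delay the cube simulates physics and falls for three seconds.
; Reset turns physics off and a timeline lerps the cube back to the transform saved at BeginPlay.
; A Ready flag tracks the cycle but is never checked before activation, and debug prints announce each stage.
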(event OnComponentBeginOverlap(Box)
  (params (OverlappedComponent :type Primitive%20Component%20Object%20Reference) (OtherActor :type Actor%20Object%20Reference) (OtherComp :type Primitive%20Component%20Object%20Reference) (OtherBodyIndex :type Integer) (bFromSweep :type Boolean) (SweepResult :type Hit%20Result%20Structure%20%28by%20ref%29))
  (Utilities|Casting|CastToCoding1ThirdPersonCustom OtherActor) ; Did player step on platform?
  (CallFunction|Activate))

(event Custom|Activate
  (Development|PrintString "One second left" true true "(R=1.000000,G=0.152066,B=0.098981,A=1.000000)")
  (Variables|Default|SetReady false)
  (Utilities|FlowControl|Delay 1.0)
  (CallFunction|Drop))

(event Custom|Drop
  (Development|PrintString "Dropping!" true true "(R=1.000000,G=0.121527,B=0.121527,A=1.000000)")
  (Physics|SetSimulatePhysics (Variables|Default|GetCube) true)
  (Utilities|FlowControl|Delay 3.0)
  (CallFunction|Reset))

(event Custom|Reset
  (Development|PrintString "Resetting")
  (Variables|Default|SetResetTransform (Transformation|GetWorldTransform (Variables|Default|GetCube)))
  (Physics|SetSimulatePhysics (Variables|Default|GetCube) false)
  (bind _newtrack_0 (Timeline|GoBackToStart PlayFromStart)
    (:Update
      (Transformation|SetWorldLocationAndRotation (Variables|Default|GetCube) (.location (Math|Transform|Lerp(Transform) (Variables|Default|GetResetTransform) (Variables|Default|GetStartingTransform) _newtrack_0)) (.rotation (Math|Transform|Lerp(Transform) (Variables|Default|GetResetTransform) (Variables|Default|GetStartingTransform) _newtrack_0)) false false))
    (:Finished
      (Variables|Default|SetReady true))))

(event EventBeginPlay
  (Variables|Default|SetStartingTransform (Transformation|GetWorldTransform (Variables|Default|GetCube))))

(event Collision|EventActorBeginOverlap
  (params (OtherActor :type Actor%20Object%20Reference)))

(event EventTick
  (params (DeltaSeconds :type Float%20%28single-precision%29)))

(fn ConstructionScript)